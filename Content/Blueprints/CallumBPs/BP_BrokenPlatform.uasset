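; Breakable platform that shatters its Geometry Collection when the test third-person character enters its box trigger.
; On first overlap, a DoOnce turns on physics simulation and applies a small radial impulse with strain at a fixed literal origin.
; Both Sequence outputs feed that same DoOnce, so the second is redundant.
; BeginPlay also applies a one-off impulse to the collection, independent of the trigger.
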(event `self.ReceiveBeginPlay`
  (`PrimitiveComponent.AddImpulse` (`self.GeometryCollection`) (1000.0 1000.0 1000.0) "None" false))

(event `self.Box.OnComponentBeginOverlap`
  (params (OverlappedComponent :type "PrimitiveComponent Object Reference") (OtherActor :type "Actor Object Reference") (OtherComp :type "PrimitiveComponent Object Reference") (OtherBodyIndex :type Integer) (bFromSweep :type Boolean) (SweepResult :type "HitResult Structure (by ref)"))
  (bind _geometrycollection (`self.GeometryCollection`))
  (bind _asbp_third_person_callum_test (cast `/Game/Blueprints/CallumBPs/BP_ThirdPersonCallumTest` OtherActor))
  (`|ExecutionSequence`
    (:`then_0`
      _)
    (:`then_1`
      _))
  (`/Engine/EditorBlueprintResources/StandardMacros.DoOnce` false
    (:`Completed`
      (`PrimitiveComponent.SetSimulatePhysics` _geometrycollection true)
      (`PhysicsObjectBlueprintLibrary.ApplyRadialImpulse` _geometrycollection (0.0 0.0 35.0) 20.0 1000.0 "RIF_Constant" true))))

(fn `UserConstructionScript`)