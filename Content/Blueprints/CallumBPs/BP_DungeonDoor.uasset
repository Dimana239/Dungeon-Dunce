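; Dungeon door behind bars that the player opens in two stages: the bars first, then the keyed door.
; BarsOpen, not called within this Blueprint, raises the bars on a timeline and sets BarsGone when finished.
; PrimaryAction then checks HasKey on BP_FirstPersonCharacter and calls DoorOpen, which swings the door open on a second timeline.
; Blocked attempts only print rattle or jiggle debug messages.
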(event `DoorOpen`
  (bind (_direction _newtrack_0) (`Timeline|Timeline_0` :!via `PlayFromStart`)
    (:`Update`
      (`SceneComponent.K2_SetRelativeRotation` (`self.Door`) (`KismetMathLibrary.MakeRotator` 0.0 0.0 (`KismetMathLibrary.Lerp` 0.0 90.0 _newtrack_0)) false false))))

(event `BarsOpen`
  (bind (_direction _bars) (`Timeline|Timeline` :!via `PlayFromStart`)
    (:`Update`
      (`SceneComponent.K2_SetRelativeLocation` (`self.Bars`) (`KismetMathLibrary.MakeVector` 100.0 20.0 (`KismetMathLibrary.Lerp` 0.0 300.0 _bars)) false false))
    (:`Finished`
      (set `self.BarsGone` true))))

(event `self.PrimaryAction`
  (if (`self.BarsGone`)
    (bind _returnvalue (`GameplayStatics.GetActorOfClass` "/Game/DungeonDunce/FirstPerson/Blueprints/BP_FirstPersonCharacter.BP_FirstPersonCharacter_C"))
    (if (`/Game/DungeonDunce/FirstPerson/Blueprints/BP_FirstPersonCharacter.hasKey` _returnvalue)
      (`self.DoorOpen`)
      (else
        (`KismetSystemLibrary.PrintString` "Jiggle Door Handle")))
    (else
      (`KismetSystemLibrary.PrintString` "Rattle Bars"))))

(fn `UserConstructionScript`
  (`parent.UserConstructionScript`))