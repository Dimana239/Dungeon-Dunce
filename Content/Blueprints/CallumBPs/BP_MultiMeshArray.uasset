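; BP_MultiMeshArray is a construction-script tool that lays out a straight array of repeated meshes.
; It adds NumberOfUnits instances to a Hierarchical Instanced Static Mesh component, spaced by Distance along the X, Y or Z axis chosen by AxisToggle.
; Offset shifts the index range, moving the whole row in whole-step increments, and each instance takes the HISM component's relative rotation.
; The event graph holds no active logic.
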(fn `UserConstructionScript`
  (bind _offset (`self.Offset`))
  (bind _distance (`self.Distance`))
  (bind _hism (`self.HISM`))
  (bind _relativerotation (`SceneComponent.RelativeRotation` _hism))
  (for _index (range _offset (+ (- (`self.Number of Units`) (- 1 _offset)) 1))
    (switch `/Game/Blueprints/CallumBPs/E_AxisSwitch` (`self.AxisToggle`)
      (:`NewEnumerator0`
        (`InstancedStaticMeshComponent.AddInstance` _hism (`KismetMathLibrary.MakeTransform` (`KismetMathLibrary.MakeVector` (* _index _distance)) _relativerotation) false))
      (:`NewEnumerator1`
        (`InstancedStaticMeshComponent.AddInstance` (`self.HISM`) (`KismetMathLibrary.MakeTransform` (`KismetMathLibrary.MakeVector` 0.0 (* _index _distance)) _relativerotation) false))
      (:`NewEnumerator2`
        (`InstancedStaticMeshComponent.AddInstance` (`self.HISM`) (`KismetMathLibrary.MakeTransform` (`KismetMathLibrary.MakeVector` 0.0 0.0 (* _index _distance)) _relativerotation) false)))))