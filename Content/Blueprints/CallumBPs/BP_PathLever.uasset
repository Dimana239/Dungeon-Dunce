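; BP_PathLever is a trigger that briefly reveals the safe platforms when BP_ThirdPersonCallumTest overlaps its Box.
; It gathers every BP_SafePlatform and uses a delayed loop to attach a level-up particle to each in turn, storing the emitters in ParticleRefArray.
; After a short pause, a second delayed loop destroys those emitters one by one.
; Two earlier loop attempts remain in the graph but never run.
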(event `self.Box.OnComponentBeginOverlap`
  (params (OverlappedComponent :type "PrimitiveComponent Object Reference") (OtherActor :type "Actor Object Reference") (OtherComp :type "PrimitiveComponent Object Reference") (OtherBodyIndex :type Integer) (bFromSweep :type Boolean) (SweepResult :type "HitResult Structure (by ref)"))
  (cast `/Game/ThirdPerson/Blueprints/BP_ThirdPersonCallumTest` OtherActor)
  (bind _outactors (`GameplayStatics.GetAllActorsOfClass` "/Game/Blueprints/CallumBPs/BP_SafePlatform.BP_SafePlatform_C"))
  (bind (_arrayelement _arrayindex) (`/Game/Blueprints/CallumBPs/BPML_Test.For Each Loop With Delay` _outactors 1.0)
    (:`LoopBody`
      (bind _returnvalue (`GameplayStatics.SpawnEmitterAttached` "/Game/InfinityBladeEffects/Effects/FX_Mobile/Misc/P_levelUp_Detail.P_levelUp_Detail" (`/Game/Blueprints/CallumBPs/BP_SafePlatform.DefaultSceneRoot` _arrayelement)))
      (`KismetArrayLibrary.Array_Set` (`self.ParticleRefArray`) _arrayindex _returnvalue true))
    (:`Completed`
      (`KismetSystemLibrary.Delay` 2.0)
      (bind _arrayelement_2 (`/Game/Blueprints/CallumBPs/BPML_Test.For Each Loop With Delay` (`self.ParticleRefArray`) 0.5)
        (:`LoopBody`
          (`ActorComponent.K2_DestroyComponent` _arrayelement_2))))))

(fn `UserConstructionScript`)