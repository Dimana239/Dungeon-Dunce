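; Torch puzzle manager that checks a number combination to open the bars of the dungeon door.
; CheckCombo appends each incoming torch number to a string, prints it, then switches on the result.
; A match on 3142 calls BarsOpen on BP_DungeonDoor, while the default branch resets every BP_Torch and clears the string.
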(event `CheckCombo`
  (params (TorchNumber :type Integer))
  (bind _returnvalue (`KismetStringLibrary.Concat_StrStr` (`self.CurrentCombo`) (`KismetStringLibrary.Conv_IntToString` TorchNumber)))
  (`KismetSystemLibrary.PrintString` _returnvalue)
  (bind _output_get (set `self.CurrentCombo` _returnvalue))
  (switch `string` _output_get
    (:`Default`
      (bind _outactors (`GameplayStatics.GetAllActorsOfClass` "/Game/Blueprints/CallumBPs/BP_Torch.BP_Torch_C"))
      (for _array_element _outactors
        (`/Game/Blueprints/CallumBPs/BP_Torch.Reset` _array_element))
      (set `self.CurrentCombo` ""))
    (:`3142`
      (bind _returnvalue_2 (`GameplayStatics.GetActorOfClass` "/Game/Blueprints/CallumBPs/BP_DungeonDoor.BP_DungeonDoor_C"))
      (`/Game/Blueprints/CallumBPs/BP_DungeonDoor.BarsOpen` _returnvalue_2))))

(fn `UserConstructionScript`)