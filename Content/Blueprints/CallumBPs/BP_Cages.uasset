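; BP_Cages is a puzzle cage that steps through four vertical positions, with its lantern lighting when it sits at the third position.
; MoveCage cycles the position index and uses a timeline to slide the cage mesh along Z.
; Further timelines drive a dynamic material's LerpValue to light or dim the lantern.
; After each light change it reports the LightOn state to BP_CageManager through CheckCages.
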(event `self.ReceiveBeginPlay`
  (bind _returnvalue (`PrimitiveComponent.CreateDynamicMaterialInstance` (`self.SM_PROP_lantern_04`) 1 "/Game/Fantastic_Village_Pack/materials/M_Master_CLR_Dyn.M_Master_CLR_Dyn" "None"))
  (set `self.DynMaterialRef` _returnvalue))

(event `MoveCage`
  (set `self.PositionIndex` (mod (+ (`self.PositionIndex`) 1) 4))
  (bind (_direction _newtrack_0) (`Timeline|Timeline` :!via `PlayFromStart`)
    (:`Update`
      (`SceneComponent.K2_SetRelativeLocation` (`self.SM_Cage`) (`KismetMathLibrary.MakeVector` 0.0 0.0 (`KismetMathLibrary.Lerp` (`self.CurrentLocation`) (* (`self.PositionIndex`) 150.0) _newtrack_0)) false false))
    (:`Finished`
      (set `self.CurrentLocation` (* (`self.PositionIndex`) 150.0))
      (if (== (`self.PositionIndex`) 2)
        (bind (_direction_2 _newtrack_0_2) (`Timeline|Timeline_0` :!via `PlayFromStart`)
          (:`Update`
            (`MaterialInstanceDynamic.SetScalarParameterValue` (`self.DynMaterialRef`) "LerpValue" _newtrack_0_2))
          (:`Finished`
            (set `self.LightOn` true)
            (bind _returnvalue (`GameplayStatics.GetActorOfClass` "/Game/Blueprints/CallumBPs/BP_CageManager.BP_CageManager_C" :!label _label))
            (`/Game/Blueprints/CallumBPs/BP_CageManager.CheckCages` _returnvalue (`self.LightOn`))))
        (elif (`self.LightOn`)
          (bind (_direction_3 _newtrack_0_3) (`Timeline|Timeline_1` :!via `PlayFromStart`)
            (:`Update`
              (`MaterialInstanceDynamic.SetScalarParameterValue` (`self.DynMaterialRef`) "LerpValue" _newtrack_0_3))
            (:`Finished`
              (set `self.LightOn` false)
              (goto _label))))))))

(fn `UserConstructionScript`)