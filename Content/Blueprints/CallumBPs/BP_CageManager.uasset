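; BP_CageManager tracks how many cage lights are on and lowers the key cage once four are lit.
; CheckCages adjusts a running count up or down by the reported light state and prints it for debugging.
; At a count of four, a DoOnce finds the BP_KeyCage1 actor and calls LowerCage on it, so the drop happens only once.
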(event `CheckCages`
  (params (LightOn :type Boolean))
  (bind _numbercageon (`self.NumberCageOn`))
  (bind _numbercageon_2 (`self.NumberCageOn`))
  (if LightOn
    (`/Engine/EditorBlueprintResources/StandardMacros.IncrementInt` _numbercageon
      (:`  `
        _))
    (else
      (`/Engine/EditorBlueprintResources/StandardMacros.DecrementInt` _numbercageon
        (:`  `
          _))))
  (`KismetSystemLibrary.PrintString` (`KismetStringLibrary.Conv_IntToString` _numbercageon_2))
  (if (== _numbercageon_2 4)
    (`/Engine/EditorBlueprintResources/StandardMacros.DoOnce` false
      (:`Completed`
        (bind _returnvalue (`GameplayStatics.GetActorOfClass` "/Game/Blueprints/CallumBPs/BP_KeyCage1.BP_KeyCage1_C"))
        (`/Game/Blueprints/CallumBPs/BP_KeyCage1.LowerCage` _returnvalue)
        (`KismetSystemLibrary.PrintString` "LOWERING")))))

(fn `UserConstructionScript`)