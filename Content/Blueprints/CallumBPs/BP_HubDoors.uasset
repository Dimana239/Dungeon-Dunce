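; BP_HubDoors is an interactable hub door that plays a short cinematic and then loads another level.
; On PrimaryAction it stops player movement, hides the first-person character and blends the view to the door actor.
; A timeline swings the door open 90 degrees, then MoveComponentTo pushes ZoomCamera through the doorway.
; When that move completes, it opens the level named by the OpenLevel variable.
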(event `self.PrimaryAction`
  (bind _returnvalue (`GameplayStatics.GetPlayerController` 0))
  (`Controller.StopMovement` _returnvalue)
  (bind _returnvalue_2 (`GameplayStatics.GetActorOfClass` "/Game/DungeonDunce/FirstPerson/Blueprints/BP_FirstPersonCharacter.BP_FirstPersonCharacter_C"))
  (`self.SetActorHiddenInGame` _returnvalue_2 true)
  (`PlayerController.SetViewTargetWithBlend` _returnvalue self 0.5 "VTBlend_Linear" 0.0 false)
  (`KismetSystemLibrary.Delay` 0.5)
  (`self.MoveCamera`))

(event `MoveCamera`
  (bind (_direction _newtrack_0) (`Timeline|Timeline` :!via `PlayFromStart`)
    (:`Update`
      (`SceneComponent.K2_SetRelativeRotation` (`self.Door`) (`KismetMathLibrary.MakeRotator` 0.0 0.0 (`KismetMathLibrary.Lerp` 0.0 -90.0 _newtrack_0)) false false))
    (:`Finished`
      (`KismetSystemLibrary.Delay` 0.2)
      (`KismetSystemLibrary.MoveComponentTo` (`self.ZoomCamera`) (100.0 -300.0 150.0) (struct :`Yaw` -90.0) false true 1.0)
      (`GameplayStatics.OpenLevel` (`self.OpenLevel`)))))

(fn `UserConstructionScript`
  (`parent.UserConstructionScript`))