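; BP_Torch is an interactable puzzle torch that switches from red fire to blue when used.
; PrimaryAction ignores input while moving, otherwise UseTorch tilts the brazier by timeline, then swaps fire, sparks and striker crystal material.
; Check then reports TorchNumber to BP_TorchManager's CheckCombo.
; A separate Reset event reverses the tilt and restores red without a check; an older combined toggle graph is left unconnected.
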(event `self.PrimaryAction`
  (if (`self.IsMoving`)
    (`KismetSystemLibrary.PrintString` "Slow ya roll buckaroo")
    (else
      (`self.UseTorch`))))

(event `UseTorch`
  (bind _redfire (`self.RedFire`))
  (if (`self.isRed`)
    (set `self.IsMoving` true)
    (bind (_direction _newtrack_0) (`Timeline|Timeline_0` :!via `PlayFromStart`)
      (:`Update`
        (`SceneComponent.K2_SetRelativeRotation` (`self.SM_BrazierTorch`) (`KismetMathLibrary.MakeRotator` 0.0 (`KismetMathLibrary.Lerp` 0.0 40.0 _newtrack_0)) false false))
      (:`Finished`
        (set `self.IsMoving` false)
        (`SceneComponent.SetHiddenInGame` (`self.BlueFire`) false false)
        (`KismetSystemLibrary.Delay` 0.1)
        (`SceneComponent.SetHiddenInGame` _redfire true false)
        (`GameplayStatics.SpawnEmitterAtLocation` "/Game/InfinityBladeEffects/Effects/FX_Monsters/FX_Monster_Ausar/P_AU_Taunt_Bluesparks.P_AU_Taunt_Bluesparks" (`SceneComponent.K2_GetComponentLocation` _redfire))
        (`PrimitiveComponent.SetMaterial` (`self.Striker`) 0 "/Game/DreamscapeSeries/DreamscapeTower/Materials/Crystals/MI_Crystal_Base_Blue.MI_Crystal_Base_Blue")
        (set `self.isRed` false)
        (`self.Check`)))))

(event `Reset`
  (bind _bluefire (`self.BlueFire`))
  (if (not (`self.isRed`))
    (set `self.IsMoving` true)
    (bind (_direction _newtrack_0) (`Timeline|Timeline_1` :!via `ReverseFromEnd`)
      (:`Update`
        (`SceneComponent.K2_SetRelativeRotation` (`self.SM_BrazierTorch`) (`KismetMathLibrary.MakeRotator` 0.0 (`KismetMathLibrary.Lerp` 0.0 40.0 _newtrack_0)) false false))
      (:`Finished`
        (set `self.IsMoving` false)
        (`SceneComponent.SetHiddenInGame` (`self.RedFire`) false false)
        (`KismetSystemLibrary.Delay` 0.1)
        (`SceneComponent.SetHiddenInGame` _bluefire true false)
        (`GameplayStatics.SpawnEmitterAtLocation` "/Game/InfinityBladeEffects/Effects/FX_Monsters/FX_Monster_Ausar/P_AU_Taunt_sparks.P_AU_Taunt_sparks" (`SceneComponent.K2_GetComponentLocation` _bluefire))
        (`PrimitiveComponent.SetMaterial` (`self.Striker`) 0 "/Game/DreamscapeSeries/DreamscapeTower/Materials/Crystals/MI_Crystal_Base_Red.MI_Crystal_Base_Red")
        (set `self.isRed` true)))))

(fn `Check`
  (bind _returnvalue (`GameplayStatics.GetActorOfClass` "/Game/Blueprints/CallumBPs/BP_TorchManager.BP_TorchManager_C"))
  (`/Game/Blueprints/CallumBPs/BP_TorchManager.CheckCombo` _returnvalue (`self.Torch Number`)))

(fn `UserConstructionScript`
  (`parent.UserConstructionScript`))