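; BP_ArtifactAlter is an interactable altar where the player places a collected artifact to light it with blue fire.
; PrimaryAction finds BP_ThirdPersonCallumTest and, if it has artifacts, deducts one, reveals the Artifact component and calls TurnOn; otherwise it prints a rejection.
; TurnOn spawns timed emitter bursts at the fire component's location, using delays before unhiding the persistent PSFXBluefire2 effect.
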(event `self.PrimaryAction`
  (bind _charref (`self.CharRef`))
  (bind _returnvalue (`GameplayStatics.GetActorOfClass` "/Game/Blueprints/CallumBPs/BP_ThirdPersonCallumTest.BP_ThirdPersonCallumTest_C"))
  (bind _output_get (set `self.CharRef` _returnvalue))
  (if (> (`/Game/Blueprints/CallumBPs/BP_ThirdPersonCallumTest.Artifacts` _output_get) 0)
    (bind _result (`/Engine/EditorBlueprintResources/StandardMacros.DecrementInt` (`/Game/Blueprints/CallumBPs/BP_ThirdPersonCallumTest.Artifacts` _charref))
      (:`  `
        (set `/Game/Blueprints/CallumBPs/BP_ThirdPersonCallumTest.Artifacts` _result _charref)
        (`SceneComponent.SetHiddenInGame` (`self.Artifact`) false false)
        (`self.TurnOn`)))
    (else
      (`KismetSystemLibrary.PrintString` "Fuck Off"))))

(event `TurnOn`
  (bind _returnvalue (`SceneComponent.K2_GetComponentLocation` (`self.PS_FX_bluefire_2`)))
  (`GameplayStatics.SpawnEmitterAtLocation` "/Game/InfinityBladeEffects/Effects/FX_Monsters/FX_Monster_Ausar/P_AU_Trap_Target.P_AU_Trap_Target" (+ _returnvalue (0.0 0.0 50.0)) (struct :`Roll` 180.0))
  (`KismetSystemLibrary.Delay` 2.75)
  (`GameplayStatics.SpawnEmitterAtLocation` "/Game/InfinityBladeEffects/Effects/FX_Monsters/FX_Monster_Ausar/P_AU_Taunt_Bluesparks.P_AU_Taunt_Bluesparks" (+ _returnvalue (0.0 0.0 20.0)) (struct) (6.0 6.0 6.0))
  (`KismetSystemLibrary.Delay` 0.1)
  (`SceneComponent.SetHiddenInGame` (`self.PS_FX_bluefire_2`) false false))

(fn `UserConstructionScript`
  (`parent.UserConstructionScript`))