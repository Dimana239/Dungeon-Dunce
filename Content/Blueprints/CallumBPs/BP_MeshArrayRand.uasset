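; Editor-configurable array actor that lays out a row of randomly chosen static meshes along a selected X, Y or Z axis.
; The construction script loops over an offset index range, spacing units by Distance and copying the InstancedStaticMesh component's rotation.
; Each unit gets its own new instanced mesh component rather than sharing one, with an unseeded random pick from StaticMeshArray, so the layout re-rolls on every reconstruction.
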(fn `UserConstructionScript`
  (bind _offset (`self.Offset`))
  (bind _distance (`self.Distance`))
  (bind _relativerotation (`SceneComponent.RelativeRotation` (`self.InstancedStaticMesh`)))
  (for _index (range _offset (+ (- (`self.Number of Units`) (- 1 _offset)) 1))
    (switch `/Game/Blueprints/CallumBPs/E_AxisSwitch` (`self.AxisToggle`)
      (:`NewEnumerator0`
        (bind _returnvalue (`AddComponent|NODE_AddInstancedStaticMeshComponent-0` :`RelativeTransform` (`KismetMathLibrary.MakeTransform` (`KismetMathLibrary.MakeVector` (* _index _distance)) _relativerotation)))
        (`StaticMeshComponent.SetStaticMesh` _returnvalue (`|GetArrayItem` (`self.StaticMeshArray`) (`KismetMathLibrary.RandomIntegerInRange` 0 (- (`self.Number of Meshs`) 1))))
        (`InstancedStaticMeshComponent.AddInstance` _returnvalue (`InstancedStaticMeshComponent.GetInstanceTransform` _returnvalue 0 false) false))
      (:`NewEnumerator1`
        (bind _returnvalue_2 (`AddComponent|NODE_AddInstancedStaticMeshComponent-1` :`RelativeTransform` (`KismetMathLibrary.MakeTransform` (`KismetMathLibrary.MakeVector` 0.0 (* _index _distance)) _relativerotation)))
        (`StaticMeshComponent.SetStaticMesh` _returnvalue_2 (`|GetArrayItem` (`self.StaticMeshArray`) (`KismetMathLibrary.RandomIntegerInRange` 0 (- (`self.Number of Meshs`) 1))))
        (`InstancedStaticMeshComponent.AddInstance` _returnvalue_2 (`InstancedStaticMeshComponent.GetInstanceTransform` _returnvalue_2 0 false) false))
      (:`NewEnumerator2`
        (bind _returnvalue_3 (`AddComponent|NODE_AddInstancedStaticMeshComponent-2` :`RelativeTransform` (`KismetMathLibrary.MakeTransform` (`KismetMathLibrary.MakeVector` 0.0 0.0 (* _index _distance)) _relativerotation)))
        (`StaticMeshComponent.SetStaticMesh` _returnvalue_3 (`|GetArrayItem` (`self.StaticMeshArray`) (`KismetMathLibrary.RandomIntegerInRange` 0 (- (`self.Number of Meshs`) 1))))
        (`InstancedStaticMeshComponent.AddInstance` _returnvalue_3 (`InstancedStaticMeshComponent.GetInstanceTransform` _returnvalue_3 0 false) false)))))