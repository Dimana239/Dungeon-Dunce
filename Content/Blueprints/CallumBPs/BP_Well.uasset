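; BP_Well is a multi-step interactable well puzzle that ends by revealing a bird statue and spawning a BP_Striker.
; PrimaryAction advances StepIndex, first consuming the player's handle to show it on the well.
; The next use cranks the handle through a Timeline with attached audio and reveals the bucket behind a fade to black.
; The last repositions the bucket after another fade, whose widget is never removed here.
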(event `self.PrimaryAction`
  (switch `int` (`self.StepIndex`)
    (:`Default`
      (`KismetSystemLibrary.PrintString` "I think I'm done here."))
    (:`0`
      (bind _asbp_first_person_character (cast `/Game/DungeonDunce/FirstPerson/Blueprints/BP_FirstPersonCharacter` (`GameplayStatics.GetPlayerCharacter` 0)))
      (if (`/Game/DungeonDunce/FirstPerson/Blueprints/BP_FirstPersonCharacter.hasHandle` _asbp_first_person_character)
        (`SceneComponent.SetHiddenInGame` (`self.SM_PROP_well_handle`) false false)
        (set `/Game/DungeonDunce/FirstPerson/Blueprints/BP_FirstPersonCharacter.hasHandle` false _asbp_first_person_character)
        (`/Engine/EditorBlueprintResources/StandardMacros.IncrementInt` (`self.StepIndex`))))
    (:`1`
      (`self.MoveHandle`)
      (`/Engine/EditorBlueprintResources/StandardMacros.IncrementInt` (`self.StepIndex`)))
    (:`2`
      (`self.MoveBucket`)
      (`/Engine/EditorBlueprintResources/StandardMacros.IncrementInt` (`self.StepIndex`)))))

(event `MoveHandle`
  (`|ExecutionSequence`
    (:`then_0`
      (`FMODBlueprintStatics.PlayEventAttached` "/Game/FMOD/Events/FOLEY/WoodenCrank.WoodenCrank" (`self.SM_PROP_well_handle`) "None" (0.0 0.0 0.0) "KeepRelativeOffset")
      (bind (_direction _newtrack_0) (`Timeline|Timeline`)
        (:`Update`
          (`SceneComponent.K2_SetRelativeRotation` (`self.SM_PROP_well_handle`) (`KismetMathLibrary.MakeRotator` 0.0 (`KismetMathLibrary.Lerp` 0.0 720.0 _newtrack_0)) false false))))
    (:`then_1`
      (`KismetSystemLibrary.Delay` 2.0)
      (bind _returnvalue (`|CreateWidget` "/Game/Blueprints/CallumBPs/Widget/W_FadeBlack.W_FadeBlack_C"))
      (`UserWidget.AddToViewport` _returnvalue 0)
      (`KismetSystemLibrary.Delay` 1.1)
      (`SceneComponent.SetHiddenInGame` (`self.SM_PROP_bucket_04`) false false)
      (`SceneComponent.SetHiddenInGame` (`self.SM_PROP_bucket_04_handle`) false false)
      (`KismetSystemLibrary.Delay` 1.1)
      (`Widget.RemoveFromParent` _returnvalue))))

(event `MoveBucket`
  (bind _defaultsceneroot (`self.DefaultSceneRoot`))
  (bind (_returnvalue_roll _returnvalue_pitch _returnvalue_yaw) (`KismetMathLibrary.BreakRotator` (`SceneComponent.K2_GetComponentRotation` _defaultsceneroot)))
  (bind _returnvalue (`|CreateWidget` "/Game/Blueprints/CallumBPs/Widget/W_FadeBlack.W_FadeBlack_C"))
  (`UserWidget.AddToViewport` _returnvalue 0)
  (`KismetSystemLibrary.Delay` 1.0)
  (`SceneComponent.K2_SetRelativeTransform` (`self.SM_PROP_bucket_04`) (`KismetMathLibrary.MakeTransform` (-112.0 155.0 15.0) (struct :`Pitch` -77.0 :`Yaw` -141.0) (1.25 1.25 1.25)) false false)
  (`SceneComponent.K2_SetRelativeLocationAndRotation` (`self.SM_PROP_bucket_04_handle`) (-4.0 0.0 56.0) (struct :`Pitch` -80.0) false false)
  (`SceneComponent.SetHiddenInGame` (`self.BirdStatue`) false false)
  (`|SpawnActorFromClass` "/Game/Blueprints/CallumBPs/BP_Striker.BP_Striker_C" (`KismetMathLibrary.MakeTransform` (+ (`SceneComponent.K2_GetComponentLocation` _defaultsceneroot) (-100.0 -190.0 0.0)) (`KismetMathLibrary.MakeRotator` _returnvalue_roll (+ _returnvalue_pitch -90.0) (+ _returnvalue_yaw 50.0))) "Undefined" "MultiplyWithRoot" null null))

(fn `UserConstructionScript`
  (`parent.UserConstructionScript`))