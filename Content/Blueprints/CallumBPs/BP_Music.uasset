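; BP_Music is a music actor that controls the level's main track, boss track and fire crackle ambience.
; On BeginPlay it starts the main track and, if the FireCrackle flag is set, also plays the fire audio.
; A BossTrack event stops the main track and starts the boss music in its place.
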(event `self.ReceiveBeginPlay`
  (`AudioComponent.Play` (`self.MainTrack`) 0.0)
  (if (`self.FireCrackle`)
    (`self.FireCrackleOn`)))

(event `FireCrackleOn`
  (`AudioComponent.Play` (`self.Fire`) 0.0))

(event `BossTrack`
  (`AudioComponent.Stop` (`self.MainTrack`))
  (`AudioComponent.Play` (`self.Boss`) 0.0))

(fn `UserConstructionScript`)