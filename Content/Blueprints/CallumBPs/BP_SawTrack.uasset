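; BP_SawTrack is a saw actor that travels along a spline track while its WoodmillSaw component spins.
; On BeginPlay it caches the BP_SplinePath found by GetActorOfClass, so no specific path is assigned per saw.
; A MoveObject timeline, rate-scaled by TimeToComplete, lerps distance along the spline to set the actor's location and rotation.
; A separate SawRotate timeline drives the blade's pitch through two full turns per play.
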(event `self.ReceiveBeginPlay`
  (bind _returnvalue (`GameplayStatics.GetActorOfClass` "/Game/Blueprints/CallumBPs/BP_SplinePath.BP_SplinePath_C"))
  (set `self.SplinePathRef` _returnvalue)
  (`self.MoveObject`)
  (bind (_direction _1) (`Timeline|SawRotate` :!via `PlayFromStart`)
    (:`Update`
      (`SceneComponent.K2_SetRelativeRotation` (`self.Woodmill_Saw`) (`KismetMathLibrary.MakeRotator` 0.0 (`KismetMathLibrary.Lerp` 0.0 -720.0 _1)) false false))))

(event `MoveObject`
  (bind _spline (`/Game/Blueprints/CallumBPs/BP_SplinePath.Spline` (`self.SplinePathRef`)))
  (`TimelineComponent.SetPlayRate` (`self.MoveObject_T`) (/ 1.0 (`self.TimeToComplete`)))
  (bind (_direction _newtrack_0) (`Timeline|MoveObject_T` :!via `PlayFromStart`)
    (:`Update`
      (bind _returnvalue (`KismetMathLibrary.Lerp` 0.0 (`SplineComponent.GetSplineLength` (`/Game/Blueprints/CallumBPs/BP_SplinePath.Spline` (`self.SplinePathRef`))) _newtrack_0))
      (`self.K2_SetActorTransform` (`KismetMathLibrary.MakeTransform` (`SplineComponent.GetLocationAtDistanceAlongSpline` _spline _returnvalue "World") (`SplineComponent.GetRotationAtDistanceAlongSpline` _spline _returnvalue "World"))))))

(fn `UserConstructionScript`)