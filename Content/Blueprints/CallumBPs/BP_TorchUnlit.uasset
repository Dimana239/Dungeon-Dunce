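; BP_TorchUnlit is a torch that starts unlit and can be lit once the player character has a striker.
; BeginPlay hides the RedFire and Striker components.
; PrimaryAction checks HasStriker on BP_FirstPersonCharacter, then either spawns sparks, reveals both components and sets IsLit, or prints that it is not lit.
; Once lit, PrimaryAction calls UseTorch instead.
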(event `self.ReceiveBeginPlay`
  (`SceneComponent.SetHiddenInGame` (`self.RedFire`) true false)
  (`SceneComponent.SetHiddenInGame` (`self.Striker`) true false))

(event `self.PrimaryAction`
  (if (`self.isLit`)
    (`self.UseTorch`)
    (else
      (bind _returnvalue (`GameplayStatics.GetActorOfClass` "/Game/DungeonDunce/FirstPerson/Blueprints/BP_FirstPersonCharacter.BP_FirstPersonCharacter_C"))
      (if (`/Game/DungeonDunce/FirstPerson/Blueprints/BP_FirstPersonCharacter.hasStriker` _returnvalue)
        (`GameplayStatics.SpawnEmitterAtLocation` "/Game/InfinityBladeEffects/Effects/FX_Monsters/FX_Monster_Ausar/P_AU_Taunt_sparks.P_AU_Taunt_sparks" (`SceneComponent.K2_GetComponentLocation` (`self.RedFire`)))
        (`SceneComponent.SetHiddenInGame` (`self.RedFire`) false false)
        (`SceneComponent.SetHiddenInGame` (`self.Striker`) false false)
        (set `self.isLit` true)
        (else
          (`KismetSystemLibrary.PrintString` "It's not lit"))))))

(fn `UserConstructionScript`
  (`parent.UserConstructionScript`))