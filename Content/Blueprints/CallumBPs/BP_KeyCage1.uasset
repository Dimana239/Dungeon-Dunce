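; BP_KeyCage1 is a cage holding a key that the player can collect.
; Its PrimaryAction event sets HasKey on the first-person character and destroys the key mesh and its gold sparkle effect.
; A LowerCage event plays a timeline that lerps the cage mesh downward along its relative Z axis.
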(event `self.PrimaryAction`
  (bind _returnvalue (`GameplayStatics.GetActorOfClass` "/Game/DungeonDunce/FirstPerson/Blueprints/BP_FirstPersonCharacter.BP_FirstPersonCharacter_C"))
  (set `/Game/DungeonDunce/FirstPerson/Blueprints/BP_FirstPersonCharacter.hasKey` true _returnvalue)
  (`ActorComponent.K2_DestroyComponent` (`self.low_poly_dungeon_assets_Key_001`))
  (`ActorComponent.K2_DestroyComponent` (`self.P_GoldSparkle_Bag_Lo_2`)))

(event `LowerCage`
  (bind (_direction _newtrack_0) (`Timeline|Timeline`)
    (:`Update`
      (`SceneComponent.K2_SetRelativeLocation` (`self.SM_Cage`) (`KismetMathLibrary.MakeVector` 0.0 0.0 (`KismetMathLibrary.Lerp` 0.0 -700.0 _newtrack_0)) false false))))

(fn `UserConstructionScript`
  (`parent.UserConstructionScript`))