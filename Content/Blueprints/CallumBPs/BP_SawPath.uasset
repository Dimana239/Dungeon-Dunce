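; BP_SawPath is a woodmill saw hazard that spins, travels along a straight path and damages the player.
; On BeginPlay, one timeline drives the saw's pitch through two full turns while another lerps its relative location between Start and End components.
; A Time variable sets a timeline's play rate as its reciprocal.
; Box overlap applies damage only to BP_ThirdPersonCallumTest characters.
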(event `self.ReceiveBeginPlay`
  (`TimelineComponent.SetPlayRate` (`self.Timeline_0`) (/ 1.0 (`self.Time`)))
  (`|ExecutionSequence`
    (:`then_0`
      (bind (_direction _1) (`Timeline|Timeline` :!via `PlayFromStart`)
        (:`Update`
          (`SceneComponent.K2_SetRelativeRotation` (`self.Woodmill_Saw`) (`KismetMathLibrary.MakeRotator` 0.0 (`KismetMathLibrary.Lerp` 0.0 -720.0 _1)) false false))))
    (:`then_1`
      (bind (_direction_2 _newtrack_0) (`Timeline|Timeline_0` :!via `PlayFromStart`)
        (:`Update`
          (`SceneComponent.K2_SetRelativeLocation` (`self.Woodmill_Saw`) (`KismetMathLibrary.VLerp` (`SceneComponent.RelativeLocation` (`self.Start`)) (`SceneComponent.RelativeLocation` (`self.End`)) _newtrack_0) false false))))))

(event `self.Box.OnComponentBeginOverlap`
  (params (OverlappedComponent :type "PrimitiveComponent Object Reference") (OtherActor :type "Actor Object Reference") (OtherComp :type "PrimitiveComponent Object Reference") (OtherBodyIndex :type Integer) (bFromSweep :type Boolean) (SweepResult :type "HitResult Structure (by ref)"))
  (bind _asbp_third_person_callum_test (cast `/Game/Blueprints/CallumBPs/BP_ThirdPersonCallumTest` OtherActor))
  (`GameplayStatics.ApplyDamage` _asbp_third_person_callum_test 1.0))

(fn `UserConstructionScript`)