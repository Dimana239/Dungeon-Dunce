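; BP_CageLever is an interactable lever that moves its linked cages when the primary action is triggered.
; PrimaryAction plays the Pull_Lever event at the lever's location, and a timeline lerps the lever's roll to animate the pull.
; It also calls MoveCage on every entry in the CageRef array at once, without waiting for the animation to finish.
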(event `self.PrimaryAction`
  (`|ExecutionSequence`
    (:`then_0`
      (bind _returnvalue (`FMODBlueprintStatics.PlayEventAtLocation` "/Game/FMOD/Events/Character_Actions/Pull_Lever.Pull_Lever" (`SceneComponent.K2_GetComponentToWorld` (`self.DefaultSceneRoot`))))
      (`FMODBlueprintStatics.EventInstanceSetPitch` _returnvalue 1.0)
      (bind (_direction _newtrack_0) (`Timeline|Timeline` :!via `PlayFromStart`)
        (:`Update`
          (`SceneComponent.K2_SetRelativeRotation` (`self.Lever`) (`KismetMathLibrary.MakeRotator` (`KismetMathLibrary.Lerp` -60.0 -120.0 _newtrack_0)) false false))))
    (:`then_1`
      (for _array_element (`self.CageRef`)
        (`/Game/Blueprints/CallumBPs/BP_Cages.MoveCage` _array_element)))))

(fn `UserConstructionScript`
  (`parent.UserConstructionScript`))