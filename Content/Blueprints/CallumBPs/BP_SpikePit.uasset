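; A spike pit trap that raises and lowers spikes on a repeating cycle and damages the player on contact.
; After a configurable start delay, a timeline lerps the Spikes' relative height and restarts after a pause each time it finishes.
; A box overlap casts to the third-person player character and applies damage, with a DoOnce reset after a short delay to limit repeat hits.
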(event `self.ReceiveBeginPlay`
  (`KismetSystemLibrary.Delay` (`self.StartDelay`))
  (bind (_direction _newtrack_0) (`Timeline|Timeline` :!via `PlayFromStart` :!label _label)
    (:`Update`
      (`SceneComponent.K2_SetRelativeLocation` (`self.Spikes`) (`KismetMathLibrary.MakeVector` 1.0 -2.0 (`KismetMathLibrary.Lerp` -80.0 25.0 _newtrack_0)) false false))
    (:`Finished`
      (`KismetSystemLibrary.Delay` 2.0)
      (goto _label :!via `PlayFromStart`))))

(event `self.Box.OnComponentBeginOverlap`
  (params (OverlappedComponent :type "PrimitiveComponent Object Reference") (OtherActor :type "Actor Object Reference") (OtherComp :type "PrimitiveComponent Object Reference") (OtherBodyIndex :type Integer) (bFromSweep :type Boolean) (SweepResult :type "HitResult Structure (by ref)"))
  (bind _asbp_third_person_callum_test (cast `/Game/ThirdPerson/Blueprints/BP_ThirdPersonCallumTest` OtherActor))
  (`/Engine/EditorBlueprintResources/StandardMacros.DoOnce` false :!label _label_2
    (:`Completed`
      (`GameplayStatics.ApplyDamage` _asbp_third_person_callum_test 1.0)
      (`KismetSystemLibrary.Delay` 0.4)
      (goto _label_2 :!via `Reset`))))

(fn `UserConstructionScript`)