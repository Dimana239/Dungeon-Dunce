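; BP_Ladder is a ladder actor that moves the player character between its two endpoints when its PrimaryAction event fires.
; It finds the BP_ThirdPersonCallumTest character by class lookup, then a FlipFlop alternately sets the capsule's world location to the End and Start components.
; Movement is an instant, unswept jump with no climbing, and the direction follows the alternation rather than the character's position.
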(event `self.PrimaryAction`
  (bind _returnvalue (`GameplayStatics.GetActorOfClass` "/Game/Blueprints/CallumBPs/BP_ThirdPersonCallumTest.BP_ThirdPersonCallumTest_C"))
  (`/Engine/EditorBlueprintResources/StandardMacros.FlipFlop`
    (:`A`
      (bind _capsulecomponent (`Character.CapsuleComponent` _returnvalue))
      (`SceneComponent.K2_SetWorldLocation` _capsulecomponent (`SceneComponent.K2_GetComponentLocation` (`self.End`)) false false))
    (:`B`
      (`SceneComponent.K2_SetWorldLocation` _capsulecomponent (`SceneComponent.K2_GetComponentLocation` (`self.Start`)) false false))))

(fn `UserConstructionScript`
  (`parent.UserConstructionScript`))