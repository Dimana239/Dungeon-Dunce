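; Boss door Blueprint that swings open once both of its altar conditions are met.
; The PrimaryAction event checks the Altar0 and Altar1 flags and calls OpenDoor only when both are true.
; OpenDoor plays a Timeline from the start, whose track interpolates the Door component's relative yaw through a quarter turn.
; Nothing in this graph sets the altar flags or closes the door.
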(event `self.PrimaryAction`
  (if (and (`self.Altar0`) (`self.Altar1`))
    (`self.OpenDoor`)))

(event `OpenDoor`
  (bind (_direction _newtrack_0) (`Timeline|Timeline` :!via `PlayFromStart`)
    (:`Update`
      (`SceneComponent.K2_SetRelativeRotation` (`self.Door`) (`KismetMathLibrary.MakeRotator` 0.0 0.0 (`KismetMathLibrary.Lerp` 0.0 -90.0 _newtrack_0)) false false))))

(fn `UserConstructionScript`
  (`parent.UserConstructionScript`))