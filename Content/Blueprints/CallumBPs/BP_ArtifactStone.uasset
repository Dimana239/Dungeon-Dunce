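; Collectible artifact stone that, when used, counts toward the player's artifacts and sends them back to the MainMap hub.
; A timeline started at BeginPlay moves the rune stone mesh vertically.
; PrimaryAction increments the count on BP_FirstPersonCharacter and copies it to MainGameInstance.
; It then hides the mesh, drops the root below its position, and after a short delay opens the hub level and destroys itself.
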(event `self.ReceiveBeginPlay`
  (`self.Movement`))

(event `Movement`
  (bind (_direction _newtrack_0) (`Timeline|Timeline` :!via `PlayFromStart`)
    (:`Update`
      (`SceneComponent.K2_SetRelativeLocation` (`self.SM_RuneStone_01_Unstable`) (`KismetMathLibrary.MakeVector` 0.0 0.0 (`KismetMathLibrary.Lerp` 50.0 90.0 _newtrack_0)) false false))))

(event `self.PrimaryAction`
  (bind _defaultsceneroot (`self.DefaultSceneRoot`))
  (bind _returnvalue (`GameplayStatics.GetActorOfClass` "/Game/DungeonDunce/FirstPerson/Blueprints/BP_FirstPersonCharacter.BP_FirstPersonCharacter_C"))
  (bind _result (`/Engine/EditorBlueprintResources/StandardMacros.IncrementInt` (`/Game/DungeonDunce/FirstPerson/Blueprints/BP_FirstPersonCharacter.Artifacts` _returnvalue))
    (:`  `
      (`KismetSystemLibrary.PrintString` (`KismetStringLibrary.Conv_IntToString` _result))
      (bind _asmain_game_instance (cast `/Game/Blueprints/CallumBPs/MainGameInstance` (`GameplayStatics.GetGameInstance`)))
      (set `/Game/Blueprints/CallumBPs/MainGameInstance.Artifacts` _result _asmain_game_instance)
      (`SceneComponent.SetHiddenInGame` (`self.SM_RuneStone_01_Unstable`) true false)
      (`SceneComponent.K2_SetWorldLocation` _defaultsceneroot (+ (`SceneComponent.K2_GetComponentLocation` _defaultsceneroot) (0.0 0.0 -500.0)) false false)
      (`KismetSystemLibrary.Delay` 3.0)
      (`self.ReturnHub`)
      (`self.K2_DestroyActor`))))

(event `ReturnHub`
  (`GameplayStatics.OpenLevel` "MainMap"))

(fn `UserConstructionScript`
  (`parent.UserConstructionScript`))