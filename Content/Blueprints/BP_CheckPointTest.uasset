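; BP_CheckPointTest is a checkpoint actor that shows its active state through the color of its fire components.
; BeginPlay gathers the six fire components into an array, which ActivateCheck and DeactivateCheck loop over to apply a teal or yellow emissive material.
; The Box overlap event casts to BP_ThirdPersonCallumTest but does nothing afterward, so neither event is triggered within this Blueprint.
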(event `self.ReceiveBeginPlay`
  (set `self.FireArray` (`|MakeArray` (`self.Fire01`) (`self.Fire02`) (`self.Fire03`) (`self.Fire04`) (`self.Fire05`) (`self.Fire06`))))

(event `ActivateCheck`
  (for _array_element (`self.FireArray`)
    (`PrimitiveComponent.SetMaterial` _array_element 0 "/Game/DungeonDunce/Models/LevelModels/Materials/M_EmissTeal.M_EmissTeal")))

(event `DeactivateCheck`
  (for _array_element (`self.FireArray`)
    (`PrimitiveComponent.SetMaterial` _array_element 0 "/Game/DungeonDunce/Models/LevelModels/Materials/emissive_yellow.emissive_yellow")))

(event `self.Box.OnComponentBeginOverlap`
  (params (OverlappedComponent :type "PrimitiveComponent Object Reference") (OtherActor :type "Actor Object Reference") (OtherComp :type "PrimitiveComponent Object Reference") (OtherBodyIndex :type Integer) (bFromSweep :type Boolean) (SweepResult :type "HitResult Structure (by ref)"))
  (cast `/Game/ThirdPerson/Blueprints/BP_ThirdPersonCallumTest` OtherActor))

(fn `UserConstructionScript`)